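; Configurable sidewalk corner piece for the Victorian Street environment, set up entirely in the Construction Script.
; SidewalkStyle selects the static mesh from corner variants of different angles, some with sloped versions; the 100° styles use meshes named 80 deg.
; Mirror flips the piece by setting a negative Y world scale, which also overrides any scale set on the mesh component.
; The Event Graph has no runtime logic.
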(event EventBeginPlay)

(event Collision|EventActorBeginOverlap
  (params (OtherActor :type Actor%20Object%20Reference)))

(event EventTick
  (params (DeltaSeconds :type Float%20%28single-precision%29)))

(fn ConstructionScript
  (bind _staticmeshcomponent (Variables|Debug|GetStaticMeshComponent))
  (bind _staticmeshcomponent_2 (Variables|Debug|GetStaticMeshComponent))
  ;[1 1 1] Mirror the mesh?
  (if (Variables|Sidewalk|GetMirror?)
    (Transformation|SetWorldScale3D _staticmeshcomponent_2 "1.000000,-1.000000,1.000000")
    (else
      (Transformation|SetWorldScale3D _staticmeshcomponent_2 "1.000000,1.000000,1.000000")))
  ;[1 1 1] Select the sidewalk mesh
  (switch Utilities|FlowControl|Switch|Switchone_sidewalks (Variables|Sidewalk|GetSidewalk%20Style)
    (:NewEnumerator1
      (Components|StaticMesh|SetStaticMesh _staticmeshcomponent "/Game/VictorianStreet/Meshes/Static/sm_sidewalk_90_deg_a.sm_sidewalk_90_deg_a"))
    (:NewEnumerator0
      (Components|StaticMesh|SetStaticMesh _staticmeshcomponent "/Game/VictorianStreet/Meshes/Static/sm_sidewalk_90_deg_b.sm_sidewalk_90_deg_b"))
    (:NewEnumerator2
      (Components|StaticMesh|SetStaticMesh _staticmeshcomponent "/Game/VictorianStreet/Meshes/Static/sm_sidewalk_80_deg_a.sm_sidewalk_80_deg_a"))
    (:NewEnumerator3
      (Components|StaticMesh|SetStaticMesh _staticmeshcomponent "/Game/VictorianStreet/Meshes/Static/sm_sidewalk_80_deg_b.sm_sidewalk_80_deg_b"))
    (:NewEnumerator4
      (Components|StaticMesh|SetStaticMesh _staticmeshcomponent "/Game/VictorianStreet/Meshes/Static/sm_sidewalk_10deg_a.sm_sidewalk_10deg_a"))))