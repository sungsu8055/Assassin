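; Configurable roof corner piece for the Victorian Street environment, built entirely in the construction script.
; Roof style and corner type enums choose the static mesh, covering square and chamfered corner variants for two roof styles.
; A material set enum assigns the two material slots, and a Mirror flag flips the mesh with a negative Y world scale.
; The event graph holds no runtime logic.
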(event EventBeginPlay)

(event Collision|EventActorBeginOverlap
  (params (OtherActor :type Actor%20Object%20Reference)))

(event EventTick
  (params (DeltaSeconds :type Float%20%28single-precision%29)))

(fn ConstructionScript
  (bind _staticmeshcomponent (Variables|Debug|GetStaticMeshComponent))
  (bind _staticmeshcomponent_2 (Variables|Debug|GetStaticMeshComponent))
  (bind _corner_type (Variables|Roof|GetCorner%20Type))
  ;[1 1 1] Mirror the mesh?
  (if (Variables|Roof|GetMirror?)
    (Transformation|SetWorldScale3D _staticmeshcomponent_2 "1.000000,-1.000000,1.000000")
    (else
      (Transformation|SetWorldScale3D _staticmeshcomponent_2 "1.000000,1.000000,1.000000")))
  ;[1 1 1] Select the mesh
  (switch Utilities|FlowControl|Switch|Switchone_roof_styles (Variables|Roof|GetRoof%20Style)
    (:NewEnumerator2
      (switch Utilities|FlowControl|Switch|Switchone_roof_corners _corner_type
        (:NewEnumerator1
          (Components|StaticMesh|SetStaticMesh _staticmeshcomponent "/Game/VictorianStreet/Meshes/Static/sm_roof_a_90deg_b.sm_roof_a_90deg_b"))
        (:NewEnumerator3
          (Components|StaticMesh|SetStaticMesh _staticmeshcomponent "/Game/VictorianStreet/Meshes/Static/sm_roof_a_90deg.sm_roof_a_90deg"))
        (:NewEnumerator0
          (Components|StaticMesh|SetStaticMesh _staticmeshcomponent "/Game/VictorianStreet/Meshes/Static/sm_roof_a_100deg.sm_roof_a_100deg"))))
    (:NewEnumerator4
      (switch Utilities|FlowControl|Switch|Switchone_roof_corners _corner_type
        (:NewEnumerator1
          (Components|StaticMesh|SetStaticMesh _staticmeshcomponent "/Game/VictorianStreet/Meshes/Static/sm_roof_b_90deg_b.sm_roof_b_90deg_b"))
        (:NewEnumerator3
          (Components|StaticMesh|SetStaticMesh _staticmeshcomponent "/Game/VictorianStreet/Meshes/Static/sm_roof_b_90deg.sm_roof_b_90deg"))
        (:NewEnumerator0
          (Components|StaticMesh|SetStaticMesh _staticmeshcomponent "/Game/VictorianStreet/Meshes/Static/sm_roof_b_100deg.sm_roof_b_100deg")))))
  ;[1 1 1] Select the material set
  (switch Utilities|FlowControl|Switch|Switchone_roof_materials (Variables|Roof|GetRoof%20Material%20Set)
    (:NewEnumerator1
      (Rendering|Material|SetMaterial _staticmeshcomponent 0 "/Game/VictorianStreet/Materials/Instances/mi_roof_a.mi_roof_a")
      (Rendering|Material|SetMaterial _staticmeshcomponent 1 "/Game/VictorianStreet/Materials/Instances/mi_wood_b.mi_wood_b"))
    (:NewEnumerator3
      (Rendering|Material|SetMaterial _staticmeshcomponent 0 "/Game/VictorianStreet/Materials/Instances/mi_roof_b.mi_roof_b")
      (Rendering|Material|SetMaterial _staticmeshcomponent 1 "/Game/VictorianStreet/Materials/Instances/mi_wood_b.mi_wood_b"))
    (:NewEnumerator0
      (Rendering|Material|SetMaterial _staticmeshcomponent 0 "/Game/VictorianStreet/Materials/Instances/mi_roof_c.mi_roof_c")
      (Rendering|Material|SetMaterial _staticmeshcomponent 1 "/Game/VictorianStreet/Materials/Instances/mi_roof_d.mi_roof_d"))))