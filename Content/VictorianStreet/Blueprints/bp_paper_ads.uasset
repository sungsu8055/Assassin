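; Placeable Victorian street prop that displays one of ten period paper advertisements, such as Beecham's Pills or Bowder Stone.
; The Construction Script switches on the Type variable and assigns the matching ad mesh to the static mesh component, so one Blueprint covers every poster variant.
; The Event Graph holds only disabled default events, so the actor has no runtime logic.
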(event EventBeginPlay)

(event Collision|EventActorBeginOverlap
  (params (OtherActor :type Actor%20Object%20Reference)))

(event EventTick
  (params (DeltaSeconds :type Float%20%28single-precision%29)))

(fn ConstructionScript
  (bind _staticmeshcomponent (Variables|Debug|GetStaticMeshComponent))
  ;[1 1 1] Select the appropriate mesh
  (switch Utilities|FlowControl|Switch|Switchone_paper_ads (Variables|Default|GetType)
    (:NewEnumerator3
      (Components|StaticMesh|SetStaticMesh _staticmeshcomponent "/Game/VictorianStreet/Meshes/Static/sm_ad_d.sm_ad_d"))
    (:NewEnumerator8
      (Components|StaticMesh|SetStaticMesh _staticmeshcomponent "/Game/VictorianStreet/Meshes/Static/sm_ad_h.sm_ad_h"))
    (:NewEnumerator0
      (Components|StaticMesh|SetStaticMesh _staticmeshcomponent "/Game/VictorianStreet/Meshes/Static/sm_ad_b.sm_ad_b"))
    (:NewEnumerator6
      (Components|StaticMesh|SetStaticMesh _staticmeshcomponent "/Game/VictorianStreet/Meshes/Static/sm_ad_g.sm_ad_g"))
    (:NewEnumerator1
      (Components|StaticMesh|SetStaticMesh _staticmeshcomponent "/Game/VictorianStreet/Meshes/Static/sm_ad_a.sm_ad_a"))
    (:NewEnumerator2
      (Components|StaticMesh|SetStaticMesh _staticmeshcomponent "/Game/VictorianStreet/Meshes/Static/sm_ad_c.sm_ad_c"))
    (:NewEnumerator9
      (Components|StaticMesh|SetStaticMesh _staticmeshcomponent "/Game/VictorianStreet/Meshes/Static/sm_ad_i.sm_ad_i"))
    (:NewEnumerator4
      (Components|StaticMesh|SetStaticMesh _staticmeshcomponent "/Game/VictorianStreet/Meshes/Static/sm_ad_e.sm_ad_e"))
    (:NewEnumerator5
      (Components|StaticMesh|SetStaticMesh _staticmeshcomponent "/Game/VictorianStreet/Meshes/Static/sm_ad_f.sm_ad_f"))
    (:NewEnumerator7
      (Components|StaticMesh|SetStaticMesh _staticmeshcomponent "/Game/VictorianStreet/Meshes/Static/sm_ad_j.sm_ad_j"))))