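; Configurable sign prop Blueprint for the Victorian Street content, with selectable shape and tint.
; The construction script clears material overrides so they do not carry over between meshes, then picks one of six sign meshes from SignType.
; SetColor builds a dynamic instance of the material matching that type, applies the Colorize and BaseColorTint parameters, and assigns it to the named slot when that slot exists.
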(event EventBeginPlay)

(event Collision|EventActorBeginOverlap
  (params (OtherActor :type Actor%20Object%20Reference)))

(event EventTick
  (params (DeltaSeconds :type Float%20%28single-precision%29)))

(fn ConstructionScript
  (bind _staticmeshcomponent (Variables|Debug|GetStaticMeshComponent))
  (bind _sign_type (Variables|Settings|GetSign%20Type))
  (bind _staticmeshcomponent_2 (Variables|Debug|GetStaticMeshComponent))
  ;[1 1 1] Reset materials to ensure material overides are reset when switching meshes
  (for (_ _array_index) (Rendering|Material|GetMaterials _staticmeshcomponent_2)
    (Rendering|Material|SetMaterial _staticmeshcomponent_2 _array_index 0))
  ;[1 1 1] Select the sign mesh
  (switch int _sign_type
    (:Default
      (Components|StaticMesh|SetStaticMesh _staticmeshcomponent "/Game/VictorianStreet/Meshes/Static/sm_sign_a.sm_sign_a" :!label _label))
    (:0
      (goto _label))
    (:1
      (Components|StaticMesh|SetStaticMesh _staticmeshcomponent "/Game/VictorianStreet/Meshes/Static/sm_sign_b.sm_sign_b"))
    (:2
      (Components|StaticMesh|SetStaticMesh _staticmeshcomponent "/Game/VictorianStreet/Meshes/Static/sm_sign_c.sm_sign_c"))
    (:3
      (Components|StaticMesh|SetStaticMesh _staticmeshcomponent "/Game/VictorianStreet/Meshes/Static/sm_sign_d.sm_sign_d"))
    (:4
      (Components|StaticMesh|SetStaticMesh _staticmeshcomponent "/Game/VictorianStreet/Meshes/Static/sm_sign_e.sm_sign_e"))
    (:5
      (Components|StaticMesh|SetStaticMesh _staticmeshcomponent "/Game/VictorianStreet/Meshes/Static/sm_sign_f.sm_sign_f")))
  (CallFunction|SetColor _sign_type))

(fn SetColor
  (params (Index :type Integer))
  (bind _staticmeshcomponent (Variables|Debug|GetStaticMeshComponent))
  (bind _slot_a (Variables|Default|Getslot_a))
  (if (Class|MeshComponent|IsMaterialSlotNameValid _staticmeshcomponent _slot_a)
    (bind _returnvalue (Rendering|Material|CreateDynamicMaterialInstance (Utilities|Array|Get(acopy) (Variables|Default|GetMaterials) Index) :!class /Script/Engine.KismetMaterialLibrary))
    (Rendering|Material|SetScalarParameterValue _returnvalue "Colorize" (Variables|Settings|GetColorize) :!class /Script/Engine.MaterialInstanceDynamic)
    (Rendering|Material|SetVectorParameterValue _returnvalue "BaseColorTint" (Variables|Settings|GetColor) :!class /Script/Engine.MaterialInstanceDynamic)
    (Rendering|Material|SetMaterialbyName _staticmeshcomponent _slot_a _returnvalue)))