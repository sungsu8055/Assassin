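; Roof window prop for the Victorian street set, offering three selectable visual styles.
; The construction script switches on the Style variable and assigns wall, trim and roof materials to several slots of the static mesh.
; Each style swaps between stone and block, or clay and brick looks with matching roof materials.
; It has no runtime logic, as the event graph holds only disabled default nodes.
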(event EventBeginPlay)

(event Collision|EventActorBeginOverlap
  (params (OtherActor :type Actor%20Object%20Reference)))

(event EventTick
  (params (DeltaSeconds :type Float%20%28single-precision%29)))

(fn ConstructionScript
  (bind _staticmeshcomponent (Variables|Debug|GetStaticMeshComponent))
  ;[1 1 1] Select materials
  (switch Utilities|FlowControl|Switch|Switchone_roof_window_styles (Variables|Style|GetStyle)
    (:NewEnumerator1
      (Rendering|Material|SetMaterial _staticmeshcomponent 0 "/Game/VictorianStreet/Materials/Instances/mi_stone_wall_a.mi_stone_wall_a")
      (Rendering|Material|SetMaterial _staticmeshcomponent 1 "/Game/VictorianStreet/Materials/Instances/mi_block_wall_a.mi_block_wall_a")
      (Rendering|Material|SetMaterial _staticmeshcomponent 2 "/Game/VictorianStreet/Materials/Instances/mi_block_wall_a.mi_block_wall_a")
      (Rendering|Material|SetMaterial _staticmeshcomponent 5 "/Game/VictorianStreet/Materials/Instances/mi_roof_d.mi_roof_d")
      (Rendering|Material|SetMaterial _staticmeshcomponent 6 "/Game/VictorianStreet/Materials/Instances/mi_roof_c.mi_roof_c"))
    (:NewEnumerator3
      (Rendering|Material|SetMaterial _staticmeshcomponent 0 "/Game/VictorianStreet/Materials/Instances/mi_clay.mi_clay")
      (Rendering|Material|SetMaterial _staticmeshcomponent 1 "/Game/VictorianStreet/Materials/Instances/mi_brick_wall_a.mi_brick_wall_a")
      (Rendering|Material|SetMaterial _staticmeshcomponent 2 "/Game/VictorianStreet/Materials/Instances/mi_brick_wall_a.mi_brick_wall_a")
      (Rendering|Material|SetMaterial _staticmeshcomponent 5 "/Game/VictorianStreet/Materials/Instances/mi_wood_b.mi_wood_b")
      (Rendering|Material|SetMaterial _staticmeshcomponent 6 "/Game/VictorianStreet/Materials/Instances/mi_roof_a.mi_roof_a"))
    (:NewEnumerator0
      (Rendering|Material|SetMaterial _staticmeshcomponent 0 "/Game/VictorianStreet/Materials/Instances/mi_clay.mi_clay")
      (Rendering|Material|SetMaterial _staticmeshcomponent 1 "/Game/VictorianStreet/Materials/Instances/mi_brick_wall_b.mi_brick_wall_b")
      (Rendering|Material|SetMaterial _staticmeshcomponent 2 "/Game/VictorianStreet/Materials/Instances/mi_brick_wall_b.mi_brick_wall_b")
      (Rendering|Material|SetMaterial _staticmeshcomponent 5 "/Game/VictorianStreet/Materials/Instances/mi_wood_b.mi_wood_b")
      (Rendering|Material|SetMaterial _staticmeshcomponent 6 "/Game/VictorianStreet/Materials/Instances/mi_roof_b.mi_roof_b"))))