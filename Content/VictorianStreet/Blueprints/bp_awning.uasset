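; Victorian street awning prop that is built entirely in the construction script, with a selectable Short or Tall type.
; It adds the matching static mesh, scales it along Y by ScaleY and offsets its location to suit the new width.
; SetColorShort or SetColorTall then applies a dynamic instance of that type's material to the named slot, with adjustable hue shift and desaturation.
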(event EventBeginPlay)

(event Collision|EventActorBeginOverlap
  (params (OtherActor :type Actor%20Object%20Reference)))

(event EventTick
  (params (DeltaSeconds :type Float%20%28single-precision%29)))

(fn ConstructionScript
  (bind _scale_y (Variables|Settings|GetScale%20Y))
  (bind _returnvalue (Math|Vector|MakeVector 1.0 _scale_y 1.0))
  (bind _returnvalue_2 (* 2.5e+02 _scale_y))
  (bind _returnvalue_3 (/ _returnvalue_2 2.0))
  (bind _returnvalue_4 (+ -125.0 _returnvalue_3))
  (bind _returnvalue_5 (Math|Vector|MakeVector 0.0 _returnvalue_4 0.0))
  (bind _returnvalue_6 (Math|Transform|MakeTransform _returnvalue_5 "0, 0, 0" _returnvalue))
  ;[1 1 1] Select the type of awning
  (switch Utilities|FlowControl|Switch|Switchone_awning (Variables|Settings|GetType)
    (:NewEnumerator1
      (bind _returnvalue_7 (AddComponent|AddStaticMeshComponent false _returnvalue_6))
      ;[1 1 1] Set the color
      (CallFunction|SetColorShort _returnvalue_7))
    (:NewEnumerator0
      (bind _returnvalue_8 (AddComponent|AddStaticMeshComponent false _returnvalue_6))
      (CallFunction|SetColorTall _returnvalue_8))))

(fn SetColorShort
  (params (Mesh :type Static%20Mesh%20Component%20Object%20Reference))
  (bind _slot_a (Variables|Default|Getslot_a))
  (if (Class|MeshComponent|IsMaterialSlotNameValid Mesh _slot_a)
    (bind _returnvalue (Rendering|Material|CreateDynamicMaterialInstance "/Game/VictorianStreet/Materials/Instances/mi_awning_a.mi_awning_a" :!class /Script/Engine.KismetMaterialLibrary))
    (Rendering|Material|SetScalarParameterValue _returnvalue "Hue Shift" (Variables|Settings|GetHue%20Shift) :!class /Script/Engine.MaterialInstanceDynamic)
    (Rendering|Material|SetScalarParameterValue _returnvalue "Desaturation" (Variables|Settings|GetDesaturation) :!class /Script/Engine.MaterialInstanceDynamic)
    (Rendering|Material|SetMaterialbyName Mesh _slot_a _returnvalue)))

(fn SetColorTall
  (params (Mesh :type Static%20Mesh%20Component%20Object%20Reference))
  (bind _slot_a (Variables|Default|Getslot_a))
  (if (Class|MeshComponent|IsMaterialSlotNameValid Mesh _slot_a)
    (bind _returnvalue (Rendering|Material|CreateDynamicMaterialInstance "/Game/VictorianStreet/Materials/Instances/mi_awning_b.mi_awning_b" :!class /Script/Engine.KismetMaterialLibrary))
    (Rendering|Material|SetScalarParameterValue _returnvalue "Hue Shift" (Variables|Settings|GetHue%20Shift) :!class /Script/Engine.MaterialInstanceDynamic)
    (Rendering|Material|SetScalarParameterValue _returnvalue "Desaturation" (Variables|Settings|GetDesaturation) :!class /Script/Engine.MaterialInstanceDynamic)
    (Rendering|Material|SetMaterialbyName Mesh _slot_a _returnvalue)))