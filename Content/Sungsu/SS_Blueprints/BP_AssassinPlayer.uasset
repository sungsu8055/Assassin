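; Assassin player character with ledge-climbing parkour and a running slide.
; Tick traces walls, ledge heights and neighbours, auto-grabbing ledges within pelvis range and setting flags for shimmying, side/up jumps and corner turns.
; Input uses those flags to climb, jump, turn or back-launch, switching Flying/Walking modes and exchanging interface messages with the AnimInstance.
; Slide temporarily shrinks the capsule and offsets the mesh; obstacle-vault logic exists but is unconnected.
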(event Custom|GrabLedge
  (bind _walllocation (Variables|Default|GetwallLocation))
  (bind _wallnormal (Variables|Default|GetwallNormal))
  (bind _wallnormal_2 (Variables|Default|GetwallNormal))
  (bind (_x _y) (Math|Vector|BreakVector _walllocation))
  (bind _returnvalue (Math|Conversions|RotationFromXVector _wallnormal_2))
  (bind _returnvalue_2 (* _wallnormal "22.000000,22.000000, 0"))
  ;[1 1 1] 난간 잡기
  (Class|IBPParkourInterface|IBPCanGrab(Message) (Components|SkeletalMesh|GetAnimInstance (Variables|Character|GetMesh)) true)
  (Pawn|Components|CharacterMovement|SetMovementMode (Variables|Character|GetCharacterMovement) "MOVE_Flying" 0)
  (Variables|Default|SetbHangingP true)
  (Components|MoveComponentTo (Variables|Default|GetCapsuleComponent) (Math|Vector|MakeVector (+ (.x _returnvalue_2) _x) (+ (.y _returnvalue_2) _y) (- (.Z (Math|Vector|BreakVector (Variables|Default|GetheightLocation))) 1.2e+02)) (Math|Rotator|MakeRotator (.roll _returnvalue) (.pitch _returnvalue) (- (.yaw _returnvalue) 1.8e+02)) false false 0.13 false)
  (Components|Movement|StopMovementImmediately (Variables|Character|GetCharacterMovement)))

(event Custom|ExitLedge
  ;[1 1 1] 난간 놓기
  (Pawn|Components|CharacterMovement|SetMovementMode (Variables|Character|GetCharacterMovement) "MOVE_Walking" 0)
  (Class|IBPParkourInterface|IBPCanGrab(Message) (Components|SkeletalMesh|GetAnimInstance (Variables|Character|GetMesh)) false)
  (Variables|Default|SetbHangingP false))

(event Custom|JumpLedgeL
  ;[1 1 1] 측면 점프 이동
  (if (< (Input|AxisValues|GetMoveRight) 0.0)
    (if (not (Variables|Default|GetbIsJumpingLedge))
      (Pawn|Components|CharacterMovement|SetMovementMode (Variables|Character|GetCharacterMovement) "MOVE_Flying" 0)
      (Class|IBPParkourInterface|IBPJumpLeftLedge(Message) (Components|SkeletalMesh|GetAnimInstance (Variables|Character|GetMesh)) true)
      (Variables|Default|SetbIsJumpingLedge true)
      (Variables|Default|SetbHangingP true)
      (Utilities|FlowControl|Delay 0.8)
      (CallFunction|GrabLedge))))

(event Custom|TurnRightTracer
  (bind _hangingmovearrowr (Variables|Default|GethangingMoveArrowR))
  (bind _returnvalue (Transformation|GetWorldLocation _hangingmovearrowr))
  (bind _returnvalue_2 (+ (.z _returnvalue) 6e+01))
  (bind _returnvalue_3 (Math|Vector|MakeVector (.x _returnvalue) (.y _returnvalue) _returnvalue_2))
  (Components|Movement|StopMovementImmediately (Variables|Character|GetCharacterMovement))
  (bind _returnvalue_4 (Collision|SphereTraceByChannel _returnvalue_3 (+ _returnvalue_3 (* (Math|Vector|GetForwardVector _hangingmovearrowr) 7e+01)) 2e+01 "TraceTypeQuery3" false (Utilities|Array|MakeArray 0) "ForOneFrame"))
  (if _returnvalue_4
    (Variables|Default|SetbCanTurnRight false)
    (else
      (Variables|Default|SetbCanTurnRight true))))

(event Custom|JumpUpTracer
  (bind _upledgearrow (Variables|Default|GetupLedgeArrow))
  (bind _returnvalue (Transformation|GetWorldLocation _upledgearrow))
  (bind _returnvalue_2 (Collision|CapsuleTraceByChannel _returnvalue _returnvalue 2e+01 1e+02 "TraceTypeQuery3" false (Utilities|Array|MakeArray 0) "ForOneFrame"))
  (if _returnvalue_2
    (Variables|Default|SetbCanJumpUp true)
    (else
      (Variables|Default|SetbCanJumpUp false))))

(event Custom|JumpUpLedge
  (bind _returnvalue (Input|AxisValues|GetMoveRight))
  (if (and (> _returnvalue -0.1) (< _returnvalue 0.1))
    (if (Variables|Default|GetbCanJumpUp)
      (if (not (Variables|Default|GetbIsJumpingLedge))
        (Pawn|Components|CharacterMovement|SetMovementMode (Variables|Character|GetCharacterMovement) "MOVE_Flying" 0)
        (Class|IBPParkourInterface|IBPJumpUpLedge(Message) (Components|SkeletalMesh|GetAnimInstance (Variables|Character|GetMesh)) true)
        (Variables|Default|SetbIsJumpingLedge true)
        (Input|DisableInput (Game|GetPlayerController 0))))))

(event Custom|HangingTurnBack
  (bind _mesh (Variables|Character|GetMesh))
  (bind _returnvalue (Components|SkeletalMesh|GetAnimInstance _mesh))
  (if (Variables|Default|GetbHangingP)
    (Utilities|FlowControl|Gate true) ; enters at Open
    (else
      (Utilities|FlowControl|Gate true) ; enters at Close
    )))

(event Custom|HangingTurnForward
  (if (Variables|Default|GetbTurnedBack)
    (Utilities|FlowControl|Gate true) ; enters at Open
    (else
      (Utilities|FlowControl|Gate true) ; enters at Close
    )))

(event Custom|HangingBackJump
  (bind _returnvalue (Transformation|GetActorRotation))
  (if (Variables|Default|GetbTurnedBack)
    (Utilities|FlowControl|Gate true) ; enters at Open
    (else
      (Utilities|FlowControl|Gate true) ; enters at Close
    )))

(event Custom|Climb
  ;[1 1 1] 난간 오르기
  (if (not (Variables|Default|GetbIsClimbingLedge))
    (Class|IBPParkourInterface|IBPClimbLedge(Message) (Components|SkeletalMesh|GetAnimInstance (Variables|Character|GetMesh)) true)
    (Pawn|Components|CharacterMovement|SetMovementMode (Variables|Character|GetCharacterMovement) "MOVE_Flying" 0)
    (Variables|Default|SetbIsClimbingLedge true)
    (Variables|Default|SetbHangingP false)))

(event Custom|RightTracer
  (bind _hangingmovearrowr (Variables|Default|GethangingMoveArrowR))
  (bind _returnvalue (Transformation|GetWorldLocation _hangingmovearrowr))
  (bind _returnvalue_2 (Collision|CapsuleTraceByChannel _returnvalue _returnvalue 2e+01 6e+01 "TraceTypeQuery3" false (Utilities|Array|MakeArray 0) "ForOneFrame"))
  (if _returnvalue_2
    (Variables|Default|SetbMoveRight true)
    (else
      (Variables|Default|SetbMoveRight false))))

(event Custom|LeftTracer
  (bind _hangingmovearrowl (Variables|Default|GethangingMoveArrowL))
  (bind _returnvalue (Transformation|GetWorldLocation _hangingmovearrowl))
  (bind _returnvalue_2 (Collision|CapsuleTraceByChannel _returnvalue _returnvalue 2e+01 6e+01 "TraceTypeQuery3" false (Utilities|Array|MakeArray 0) "ForOneFrame"))
  (if _returnvalue_2
    (Variables|Default|SetbMoveLeft true)
    (else
      (Variables|Default|SetbMoveLeft false))))

(event Custom|LedgeMove
  ;[1 1 1] 난간 측면 이동
  (if (not (Variables|Default|GetbTurnedBack))
    (if (Variables|Default|GetbHangingP)
      (CallFunction|IBPSideMoveLedge (Input|AxisValues|GetMoveRight))
      (CallFunction|MoveinLedge)
      (else
        (Variables|Default|SetbMovingRight false)
        (Variables|Default|SetbMovingLeft false)))))

(event Custom|JumpRightTracer
  (bind _rightledgearrow (Variables|Default|GetrightLedgeArrow))
  (bind _returnvalue (Transformation|GetWorldLocation _rightledgearrow))
  (bind _returnvalue_2 (Collision|CapsuleTraceByChannel _returnvalue _returnvalue 25.0 6e+01 "TraceTypeQuery3" false (Utilities|Array|MakeArray 0) "ForOneFrame"))
  (if _returnvalue_2
    (if (Variables|Default|GetbMoveRight)
      (Variables|Default|SetbCanJumpRight false)
      (else
        (Variables|Default|SetbCanJumpRight true)))
    (else
      (Variables|Default|SetbCanJumpRight false))))

(event Custom|JumpLeftTracer
  (bind _leftledgearrow (Variables|Default|GetleftLedgeArrow))
  (bind _returnvalue (Transformation|GetWorldLocation _leftledgearrow))
  (bind _returnvalue_2 (Collision|CapsuleTraceByChannel _returnvalue _returnvalue 25.0 6e+01 "TraceTypeQuery3" false (Utilities|Array|MakeArray 0) "ForOneFrame"))
  (if _returnvalue_2
    (if (Variables|Default|GetbMoveLeft)
      (Variables|Default|SetbCanJumpLeft false)
      (else
        (Variables|Default|SetbCanJumpLeft true)))
    (else
      (Variables|Default|SetbCanJumpLeft false))))

(event Custom|TurnLeftTracer
  (bind _hangingmovearrowl (Variables|Default|GethangingMoveArrowL))
  (bind _returnvalue (Transformation|GetWorldLocation _hangingmovearrowl))
  (bind _returnvalue_2 (+ (.z _returnvalue) 6e+01))
  (bind _returnvalue_3 (Math|Vector|MakeVector (.x _returnvalue) (.y _returnvalue) _returnvalue_2))
  (Components|Movement|StopMovementImmediately (Variables|Character|GetCharacterMovement))
  (bind _returnvalue_4 (Collision|SphereTraceByChannel _returnvalue_3 (+ _returnvalue_3 (* (Math|Vector|GetForwardVector _hangingmovearrowl) 7e+01)) 2e+01 "TraceTypeQuery3" false (Utilities|Array|MakeArray 0) "ForOneFrame"))
  (if _returnvalue_4
    (Variables|Default|SetbCanTurnLeft false)
    (else
      (Variables|Default|SetbCanTurnLeft true))))

(event Custom|JumpLedgeR
  ;[1 1 1] 측면 점프 이동
  (if (> (Input|AxisValues|GetMoveRight) 0.0)
    (if (not (Variables|Default|GetbIsJumpingLedge))
      (Pawn|Components|CharacterMovement|SetMovementMode (Variables|Character|GetCharacterMovement) "MOVE_Flying" 0)
      (Class|IBPParkourInterface|IBPJumpRightLedge(Message) (Components|SkeletalMesh|GetAnimInstance (Variables|Character|GetMesh)) true)
      (Variables|Default|SetbIsJumpingLedge true)
      (Variables|Default|SetbHangingP true)
      (Utilities|FlowControl|Delay 0.8)
      (CallFunction|GrabLedge))))

(event EventBeginPlay)

(event Collision|EventActorBeginOverlap
  (params (OtherActor :type Actor%20Object%20Reference)))

(event EventTick
  (params (DeltaSeconds :type Float%20%28single-precision%29))
  ;[1 1 1] 벽 정보 측정
  (CallFunction|ForwardTracer)
  (CallFunction|HeightTracer)
  (CallFunction|JumpUpTracer)
  (if (Variables|Default|GetbHangingP)
    (Utilities|FlowControl|Sequence
      (:then_0
        (CallFunction|LeftTracer)
        (CallFunction|RightTracer)
        (CallFunction|LedgeMove)
        (CallFunction|HangingTurnBack)
        (CallFunction|HangingTurnForward)
        (CallFunction|HangingBackJump))
      (:then_1
        (if (Variables|Default|GetbMoveLeft)
          (Variables|Default|SetbCanJumpLeft false)
          (Variables|Default|SetbCanTurnLeft false)
          (else
            (CallFunction|JumpLeftTracer)
            (if (Variables|Default|GetbCanJumpLeft)
              (Variables|Default|SetbCanTurnLeft false)
              (else
                (CallFunction|TurnLeftTracer))))))
      (:then_2
        (if (Variables|Default|GetbMoveRight)
          (Variables|Default|SetbCanJumpRight false)
          (Variables|Default|SetbCanTurnRight false)
          (else
            (CallFunction|JumpRightTracer)
            (if (Variables|Default|GetbCanJumpRight)
              (Variables|Default|SetbCanTurnRight false)
              (else
                (CallFunction|TurnRightTracer)))))))))

(event EventIBPClimbLedge
  (params (bIsClimbing :type Boolean))
  ;[1 1 1] 난간 오르기
  ;;[1 1 1] 오르기 완료 상태 전환
  (Variables|Default|SetbIsClimbingLedge bIsClimbing)
  (Pawn|Components|CharacterMovement|SetMovementMode (Variables|Character|GetCharacterMovement) "MOVE_Walking" 0))

(event EventIBPJumpUpLedge
  (params (bIBPJumpup :type Boolean))
  (Variables|Default|SetbIsJumpingLedge bIBPJumpup)
  (Components|Movement|StopMovementImmediately (Variables|Character|GetCharacterMovement))
  (Variables|Default|SetbIsJumpingLedge false)
  (CallFunction|GrabLedge)
  (Input|EnableInput (Game|GetPlayerController 0)))

(event EventIBPJumpRightLedge
  (params (JumpRight :type Boolean))
  ;[1 1 1] 측면 점프 이동
  (Variables|Default|SetbIsJumpingLedge JumpRight)
  (Components|Movement|StopMovementImmediately (Variables|Character|GetCharacterMovement))
  (Variables|Default|SetbIsJumpingLedge false))

(event EventIBPJumpLeftLedge
  (params (JumpLeft :type Boolean))
  ;[1 1 1] 측면 점프 이동
  (Variables|Default|SetbIsJumpingLedge JumpLeft)
  (Components|Movement|StopMovementImmediately (Variables|Character|GetCharacterMovement))
  (Variables|Default|SetbIsJumpingLedge false))

(event Input|ActionEvents|InputActionJump
  (params (Key :type Key%20Structure :default "None"))
  (:Pressed
    (if (Variables|Default|GetbHangingP)
      (if (not (Variables|Default|GetbTurnedBack))
        (if (Variables|Default|GetbCanJumpRight)
          (if (> (Input|AxisValues|GetMoveRight) 0.0)
            (CallFunction|JumpLedgeR)
            (else
              (CallFunction|Climb :!label _label)))
          (elif (Variables|Default|GetbCanJumpLeft)
            (if (< (Input|AxisValues|GetMoveRight) 0.0)
              (CallFunction|JumpLedgeL)
              (else
                (goto _label)))
            (elif (Variables|Default|GetbCanJumpUp)
              (CallFunction|JumpUpLedge)
              (else
                (goto _label))))))
      (else
        (Character|Jump))))
  (:Released
    (Character|StopJumping)))

(event Input|KeyboardEvents|E
  (params (Key :type Key%20Structure :default "None"))
  (bind _mesh (Variables|Character|GetMesh))
  (bind _mesh_2 (Variables|Character|GetMesh))
  ;[1 1 1] 슬라이딩
  (:Pressed
    ;;[1 1 1] 슬라이딩 실행
    (if (and (> (Math|Vector|VectorLength (Variables|/Script/Engine.MovementComponent|GetVelocity (Variables|Character|GetCharacterMovement))) 1.8e+02) (not (AI|Components|NavMovement|IsFalling (Variables|Character|GetCharacterMovement))))
      ;;[1 1 1] 슬라이딩 애니메이션 실행 시 컬리전과 메쉬의 위치 값과 높이를 바닥으로 낮춤
      (Utilities|FlowControl|DoOnce false :!label _label
        (:Completed
          (Components|Capsule|SetCapsuleHalfHeight (Variables|Default|GetCapsuleComponent) 48.0 true)
          (Transformation|SetWorldLocation _mesh_2 (+ (Transformation|GetWorldLocation _mesh_2) "0.000000, 0,50.000000") false false)
          (Animation|PlayAnimMontage "/Game/Sungsu/SS_Animation/AM_AssassinSliding.AM_AssassinSliding" 1.0 "None")
          (Utilities|FlowControl|Delay 1.0)
          ;;[1 1 1] 애니메이션을 위해 조정한 컬리전 및 메쉬 값 원복
          (Components|Capsule|SetCapsuleHalfHeight (Variables|Default|GetCapsuleComponent) 9e+01 true)
          (Transformation|SetWorldLocation _mesh (- (Transformation|GetWorldLocation _mesh) "0, 0,50.000000") false false)
          (goto _label Reset))))))

(event Input|KeyboardEvents|S
  (params (Key :type Key%20Structure :default "None"))
  (bind _mesh (Variables|Character|GetMesh))
  (bind _returnvalue (Components|SkeletalMesh|GetAnimInstance _mesh))
  (:Pressed
    (Utilities|FlowControl|Gate true
      (:Exit
        (if (Variables|Default|GetbTurnedBack)
          (Variables|Default|SetbTurnedBack false)
          (Class|IBPParkourInterface|IBPTurnBack(Message) _returnvalue false)
          (CallFunction|ExitLedge)
          (else
            (Variables|Default|SetbTurnedBack true)
            (Class|IBPParkourInterface|IBPTurnBack(Message) _returnvalue true)))))))

(event Input|KeyboardEvents|A
  (params (Key :type Key%20Structure :default "None"))
  (bind _returnvalue (Game|GetPlayerController 0))
  ;[1 1 1] 벽타기 중 코너 턴
  (:Pressed
    (if (Variables|Default|GetbHangingP)
      (if (not (Variables|Default|GetbCanJumpLeft))
        (if (Variables|Default|GetbCanTurnLeft)
          (Input|DisableInput _returnvalue)
          (Animation|PlayAnimMontage "/Game/Sungsu/SS_Animation/AM_CornerLEft.AM_CornerLEft" 1.0 "None")
          (Utilities|FlowControl|Delay 1.2)
          (CallFunction|GrabLedge)
          (Utilities|FlowControl|Delay 0.2)
          (Input|EnableInput _returnvalue))))))

(event Input|KeyboardEvents|D
  (params (Key :type Key%20Structure :default "None"))
  (bind _returnvalue (Game|GetPlayerController 0))
  ;[1 1 1] 벽타기 중 코너 턴
  (:Pressed
    (if (Variables|Default|GetbHangingP)
      (if (not (Variables|Default|GetbCanJumpRight))
        (if (Variables|Default|GetbCanTurnRight)
          (Input|DisableInput _returnvalue)
          (Animation|PlayAnimMontage "/Game/Sungsu/SS_Animation/AM_CornerRight.AM_CornerRight" 1.0 "None")
          (Utilities|FlowControl|Delay 1.2)
          (CallFunction|GrabLedge)
          (Utilities|FlowControl|Delay 0.2)
          (Input|EnableInput _returnvalue))))))

(event Input|KeyboardEvents|W
  (params (Key :type Key%20Structure :default "None"))
  (:Pressed
    (Utilities|FlowControl|Gate true
      (:Exit
        (Class|IBPParkourInterface|IBPTurnBack(Message) (Components|SkeletalMesh|GetAnimInstance (Variables|Character|GetMesh)) false)
        (Variables|Default|SetbTurnedBack false)))))

(event Input|KeyboardEvents|SpaceBar
  (params (Key :type Key%20Structure :default "None"))
  (bind _returnvalue (Transformation|GetActorRotation))
  (:Pressed
    (Utilities|FlowControl|Gate true
      (:Exit
        (if (Variables|Default|GetbHangingP)
          (if (not (Variables|Default|GetbIsJumpingLedge))
            (Character|LaunchCharacter (+ (* (Transformation|GetActorForwardVector) -5e+02) "0, 0,700.000000") false false)
            (CallFunction|ExitLedge)
            (Class|IBPParkourInterface|IBPTurnBack(Message) (Components|SkeletalMesh|GetAnimInstance (Variables|Character|GetMesh)) false)
            (Variables|Default|SetbTurnedBack false)
            (Transformation|SetActorRotation (Math|Rotator|MakeRotator (.roll _returnvalue) (.pitch _returnvalue) (- (.yaw _returnvalue) 1.8e+02)))))))))

(fn ConstructionScript)

(fn ForwardTracer
  (bind _returnvalue (Transformation|GetActorLocation))
  (bind _returnvalue_2 (Transformation|GetActorRotation))
  (bind _returnvalue_3 (Math|Vector|GetForwardVector _returnvalue_2))
  (bind (_outhit _returnvalue_4) (Collision|SphereTraceByChannel _returnvalue (+ (Math|Vector|MakeVector (* (.x _returnvalue_3) 1.5e+02) (* (.y _returnvalue_3) 1.5e+02) (.z _returnvalue_3)) _returnvalue) 2e+01 "TraceTypeQuery3" false (Utilities|Array|MakeArray 0) "ForOneFrame"))
  (if _returnvalue_4
    (Variables|Default|SetwallLocation (.Location (Collision|BreakHitResult _outhit)))
    (Variables|Default|SetwallNormal (.Normal (Collision|BreakHitResult _outhit)))))

(fn HeightTracer
  (bind _returnvalue (Transformation|GetActorLocation))
  (bind _returnvalue_2 (Transformation|GetActorRotation))
  (bind _returnvalue_3 (Math|Vector|GetForwardVector _returnvalue_2))
  (bind _returnvalue_4 (+ (.z _returnvalue) 5e+02))
  (bind _returnvalue_5 (Math|Vector|MakeVector (.x _returnvalue) (.y _returnvalue) _returnvalue_4))
  (bind _returnvalue_6 (* _returnvalue_3 7e+01))
  (bind _returnvalue_7 (+ _returnvalue_5 _returnvalue_6))
  (bind (_x _y _z) (Math|Vector|BreakVector _returnvalue_7))
  (bind (_outhit _returnvalue_8) (Collision|SphereTraceByChannel _returnvalue_7 (Math|Vector|MakeVector _x _y (- _z 5e+02)) 2e+01 "TraceTypeQuery3" false (Utilities|Array|MakeArray 0) "ForOneFrame"))
  (if _returnvalue_8
    (Variables|Default|SetheightLocation (.Location (Collision|BreakHitResult _outhit)))
    (if (Math|Float|InRange(Float) (- (.z (Transformation|GetSocketLocation (Variables|Character|GetMesh) (Variables|Default|GetpelvisSocket))) (.Z (Math|Vector|BreakVector (Variables|Default|GetheightLocation)))) -5e+01 0.0)
      (if (not (or (Variables|Default|GetbIsClimbingLedge) (Variables|Default|GetbIsJumpingLedge)))
        (CallFunction|GrabLedge)))))

(fn MoveinLedge
  (bind _returnvalue (Transformation|GetActorLocation))
  (bind _returnvalue_2 (Transformation|GetActorLocation))
  (bind _returnvalue_3 (Input|AxisValues|GetMoveRight))
  (Utilities|FlowControl|Sequence
    (:then_0
      (if (Variables|Default|GetbMoveRight)
        (if (> (Input|AxisValues|GetMoveRight) 0.0)
          (Transformation|SetActorLocation (Math|Interpolation|VInterpTo _returnvalue (+ (* (Math|Vector|GetRightVector (Transformation|GetActorRotation)) 2e+01) _returnvalue) (Utilities|Time|GetWorldDeltaSeconds) 5.0) false false)
          (Variables|Default|SetbMovingRight true)
          (Variables|Default|SetbMovingLeft false))))
    (:then_1
      (if (Variables|Default|GetbMoveLeft)
        (if (< (Input|AxisValues|GetMoveRight) 0.0)
          (Transformation|SetActorLocation (Math|Interpolation|VInterpTo _returnvalue_2 (+ (* (Math|Vector|GetRightVector (Transformation|GetActorRotation)) -2e+01) _returnvalue_2) (Utilities|Time|GetWorldDeltaSeconds) 5.0) false false)
          (Variables|Default|SetbMovingRight false)
          (Variables|Default|SetbMovingLeft true))))
    (:then_2
      (if (and (> _returnvalue_3 -0.1) (< _returnvalue_3 0.1))
        (Variables|Default|SetbMovingRight false)
        (Variables|Default|SetbMovingLeft false)))))