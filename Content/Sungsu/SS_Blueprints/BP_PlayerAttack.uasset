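; Combat component for the assassin player that handles enemy targeting, lunge attacks and a placeholder guard.
; Each tick it sphere-scans for AI enemies, targets the one nearest DesiredTargetDir, and clears combat when none are in range.
; Attacking notifies the anim instance and slides the capsule to a fixed gap from the target, then enters combat, where the player keeps facing it.
; Parkour mode drops combat and restores movement-oriented rotation.
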(event Custom|PlayersGuard
  (if (Utilities|Enum|Equal(Enum) (Variables|Default|GetcombatState) "NewEnumerator1")
    (Variables|Default|SetcombatState "NewEnumerator3")
    (Development|PrintString "Guard!!" true true "(R=1.000000,G=0.906003,B=0.000000,A=1.000000)")
    (Variables|Default|SetcombatState "NewEnumerator1")))

(event Custom|PlayersAttack
  (bind _targetedenemy (Variables|Default|GettargetedEnemy))
  (bind _player (Variables|Default|Getplayer))
  (bind _returnvalue (Transformation|GetActorLocation _player))
  (bind _returnvalue_2 (Transformation|GetActorLocation _targetedenemy))
  (bind _mesh (Variables|/Script/Engine.Character|GetMesh _player))
  (bind _returnvalue_3 (- _returnvalue_2 _returnvalue))
  (bind _returnvalue_4 (Components|SkeletalMesh|GetAnimInstance _mesh))
  (bind _returnvalue_5 (Math|Rotator|MakeRotfromXY _returnvalue_3 _returnvalue_3))
  (bind _returnvalue_6 (Math|Vector|GetForwardVector _returnvalue_5))
  (Utilities|IsValid _targetedenemy
    (:Is%20Valid
      (Utilities|FlowControl|Sequence
        (:then_0
          (Class|IBPParkourInterface|IBPAttack(Message) _returnvalue_4 true)
          (bind _output_get (Variables|Default|SetbInCombat false))
          (Class|IBPParkourInterface|IBPinCombat(Message) _returnvalue_4 _output_get)
          (Variables|Default|SetcombatState "NewEnumerator2")
          (Components|MoveComponentTo (Variables|/Script/Engine.Character|GetCapsuleComponent _player) (+ _returnvalue (* _returnvalue_6 (- (Math|Vector|VectorLength _returnvalue_3) 8e+01))) (Math|Conversions|RotationFromXVector _returnvalue_6) false false 0.6 false)
          (Variables|Default|SetcombatState "NewEnumerator1")
          (Variables|/Script/Engine.CharacterMovementComponent|SetbOrientRotationToMovement (Variables|/Script/Engine.Character|GetCharacterMovement _player) false)
          (bind _output_get_2 (Variables|Default|SetbInCombat true))
          (Class|IBPParkourInterface|IBPinCombat(Message) _returnvalue_4 _output_get_2))))))

(event EventBeginPlay
  (bind _asbp_assassin_player (Utilities|Casting|CastToBP_AssassinPlayer (Components|GetOwner)))
  (Variables|Default|Setplayer _asbp_assassin_player)
  (Variables|Default|SetcombatState "NewEnumerator0"))

(event EventTick
  (params (DeltaSeconds :type Float%20%28single-precision%29))
  (bind _player (Variables|Default|Getplayer))
  (bind _player_2 (Variables|Default|Getplayer))
  (bind _returnvalue (Transformation|GetActorRotation _player))
  (Utilities|FlowControl|Sequence
    (:then_0
      (switch Utilities|FlowControl|Switch|SwitchonEBP_CombatState (Variables|Default|GetcombatState)
        (:NewEnumerator1
          (Utilities|IsValid (Variables|Default|GettargetedEnemy)
            (:Is%20Valid
              (if (Variables|Default|GetbInCombat)
                (Transformation|SetActorRotation _player (Math|Rotator|MakeRotator (.roll _returnvalue) (.pitch _returnvalue) (.yaw (Math|Rotator|FindLookatRotation (Transformation|GetActorLocation _player) (Transformation|GetActorLocation (Variables|Default|GettargetedEnemy))))))))))))
    (:then_1
      (if (Variables|/Script/Assassin.AssassinPlayer|GetbParkourMode _player_2)
        (Variables|Default|SetbInCombat false)
        (Variables|/Script/Engine.CharacterMovementComponent|SetbOrientRotationToMovement (Variables|/Script/Engine.Character|GetCharacterMovement _player_2) true)))
    (:then_2
      (CallFunction|AttackRangeTracer))))

(fn AttackRangeTracer
  (bind _desiredtargetdir (Variables|Default|GetdesiredTargetDir))
  (Variables|Default|SetnearestEnemyDistance 5e+04)
  (bind (_outactors _returnvalue) (Collision|SphereOverlapActors (Transformation|GetActorLocation (Variables|Default|Getplayer)) 4e+02 (Variables|Default|GetTargetTraceType) "/Game/Enemy/AIEnemy/AIEnemy.AIEnemy_C"))
  (if _returnvalue
    (for _array_element _outactors
      (bind _asaienemy (Utilities|Casting|CastToAIEnemy _array_element))
      (if (< (Math|Vector|VectorLength (- (Transformation|GetActorLocation _array_element) (Variables|Default|GetdesiredTargetDir))) (Variables|Default|GetnearestEnemyDistance))
        (Variables|Default|SetnearestEnemyDistance (Math|Vector|VectorLength (- (Transformation|GetActorLocation _array_element) (Variables|Default|GetdesiredTargetDir))))
        (Variables|Default|SettargetedEnemy _asaienemy)))
    (Development|PrintString "Enemy" true true "(R=1.000000,G=0.070160,B=0.000000,A=1.000000)" 0.1)
    (Class|KismetSystemLibrary|CapsuleTraceSingleforObjects _desiredtargetdir _desiredtargetdir 5e+01 4e+01 (Variables|Default|GetTargetTraceType) false 0 "ForOneFrame" true)
    (else
      (Variables|Default|SetnearestEnemyDistance 5e+04)
      (Variables|Default|SetcombatState "NewEnumerator0")
      (Variables|Default|SetbInCombat false)
      (Variables|Default|SettargetedEnemy 0))))