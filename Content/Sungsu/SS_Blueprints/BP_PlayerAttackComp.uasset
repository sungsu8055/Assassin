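; Player combat component for BP_AssassinPlayer that handles attack, guard, assassination, taking hits and death.
; Each tick it targets the overlapping enemy nearest DesiredTargetDir, faces it while in combat, and drops combat during parkour or with no overlaps.
; Attacks use MoveComponentTo to stop a fixed distance short of the target.
; Interface messages drive player and enemy reactions, while combat state decides whether incoming hits are blocked or cost HP.
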(event Custom|PlayersGuard
  (params (bInputDefence :type Boolean))
  ;[1 1 1] 방어
  (if bInputDefence
    (if (Utilities|Enum|Equal(Enum) (Variables|Default|GetplayerCombatState) "NewEnumerator1")
      (Variables|Default|SetplayerCombatState "NewEnumerator3")
      (Development|PrintString "SS : Guard!!" true true "(R=1.000000,G=0.906003,B=0.000000,A=1.000000)"))
    (else
      (Variables|Default|SetplayerCombatState "NewEnumerator1"))))

(event Custom|PlayersAttack
  (bind _targetedenemy (Variables|Default|GettargetedEnemy))
  (bind _player (Variables|Default|Getplayer))
  (bind _returnvalue (Transformation|GetActorLocation _targetedenemy))
  (bind _returnvalue_2 (Transformation|GetActorLocation _player))
  (bind _mesh (Variables|/Script/Engine.Character|GetMesh _player))
  (bind _returnvalue_3 (- _returnvalue _returnvalue_2))
  (bind _returnvalue_4 (Components|SkeletalMesh|GetAnimInstance _mesh))
  (bind _returnvalue_5 (Math|Rotator|MakeRotfromXY _returnvalue_3 _returnvalue_3))
  (bind _returnvalue_6 (Math|Vector|GetForwardVector _returnvalue_5))
  ;[1 1 1] 공격
  (Utilities|IsValid _targetedenemy
    (:Is%20Valid
      (Utilities|FlowControl|Sequence
        (:then_0
          (bind _output_get (Variables|Default|SetrandAnimNum (Math|Random|RandomIntegerinRange 0 1)))
          (Class|IBPCombatSystem|IBPAttack(Message) _targetedenemy true _output_get)
          (Class|IBPCombatSystem|IBPAttack(Message) _returnvalue_4 true _output_get)
          (bind _output_get_2 (Variables|Default|SetbInCombat false))
          (Class|IBPCombatSystem|IBPinCombat(Message) _returnvalue_4 _output_get_2)
          (Variables|Default|SetplayerCombatState "NewEnumerator2")
          (Components|MoveComponentTo (Variables|/Script/Engine.Character|GetCapsuleComponent _player) (+ _returnvalue_2 (* _returnvalue_6 (- (Math|Vector|VectorLength _returnvalue_3) 8e+01))) (Math|Conversions|RotationFromXVector _returnvalue_6) false false 0.6 false)
          (Variables|Default|SetplayerCombatState "NewEnumerator1")
          (Variables|/Script/Engine.CharacterMovementComponent|SetbOrientRotationToMovement (Variables|/Script/Engine.Character|GetCharacterMovement _player) false)
          (bind _output_get_3 (Variables|Default|SetbInCombat true))
          (Class|IBPCombatSystem|IBPinCombat(Message) _returnvalue_4 _output_get_3)
          (Development|PrintString "SS : Attack"))))))

(event Custom|PlayersAssassinate
  ;[1 1 1] 암살
  (bind _output_get (Variables|Default|SetrandAnimNum (Math|Random|RandomIntegerinRange 0 1)))
  (Class|IBPCombatSystem|IBPAssassinatedAttack(Message) (Variables|Default|GettargetedEnemy) true _output_get)
  (Class|IBPCombatSystem|IBPAssassinatedAttack(Message) (Components|SkeletalMesh|GetAnimInstance (Variables|/Script/Engine.Character|GetMesh (Variables|Default|Getplayer))) true)
  (Development|PrintString "SS : Assassinate" true true "(R=1.000000,G=0.000000,B=0.899543,A=1.000000)"))

(event EventBeginPlay
  (bind _asbp_assassin_player (Utilities|Casting|CastToBP_AssassinPlayer (Components|GetOwner)))
  (Variables|Default|Setplayer _asbp_assassin_player)
  (Variables|Default|SetplayerCombatState "NewEnumerator0")
  (Variables|Default|SetbMainWeapon false))

(event EventTick
  (params (DeltaSeconds :type Float%20%28single-precision%29))
  (bind _player (Variables|Default|Getplayer))
  (bind _player_2 (Variables|Default|Getplayer))
  (bind _returnvalue (Transformation|GetActorRotation _player))
  (Utilities|FlowControl|Sequence
    (:then_0
      (switch Utilities|FlowControl|Switch|SwitchonEBP_PlayerCombatState (Variables|Default|GetplayerCombatState)
        (:NewEnumerator1
          (Utilities|IsValid (Variables|Default|GettargetedEnemy)
            (:Is%20Valid
              (if (Variables|Default|GetbInCombat)
                (Transformation|SetActorRotation _player (Math|Rotator|MakeRotator (.roll _returnvalue) (.pitch _returnvalue) (.yaw (Math|Rotator|FindLookatRotation (Transformation|GetActorLocation _player) (Transformation|GetActorLocation (Variables|Default|GettargetedEnemy))))))))))))
    (:then_1
      (if (Variables|/Script/Assassin.AssassinPlayer|GetbParkourMode _player_2)
        (Variables|Default|SetbInCombat false)
        (Variables|/Script/Engine.CharacterMovementComponent|SetbOrientRotationToMovement (Variables|/Script/Engine.Character|GetCharacterMovement _player_2) true)))
    (:then_2
      (CallFunction|AttackRangeTracer))))

(event EventIBPDetected
  (params (bIBPDetected :type Boolean))
  (Variables|Default|SetbMainWeapon bIBPDetected))

(event EventIBPEnemyTrackingFailure
  (params (bIBPTrackingFailure :type Boolean))
  (Variables|Default|SetbMainWeapon bIBPTrackingFailure))

(event EventIBPAttack
  (params (IBPAttack :type Boolean) (animNum :type Integer))
  (bind _returnvalue (Math|Random|RandomIntegerinRange 0 1))
  (bind _player (Variables|Default|Getplayer))
  (bind _mesh (Variables|/Script/Engine.Character|GetMesh _player))
  (bind _returnvalue_2 (Components|SkeletalMesh|GetAnimInstance _mesh))
  ;[1 1 1] 피격
  (if (Utilities|Enum|Equal(Enum) (Variables|Default|GetplayerCombatState) "NewEnumerator3")
    (Class|IBPCombatSystem|IBPDefenceState(Message) (Variables|Default|GettargetedEnemy) true)
    (Class|IBPCombatSystem|IBPDefenceState(Message) _returnvalue_2 true)
    (Development|PrintString "SS : Defence")
    (else
      (bind _result (Math|Float|DecrementFloat (Variables|/Game/Sungsu/SS_Blueprints/BP_AssassinPlayer.BP_AssassinPlayer_C|GetplayerHP _player))
        (:%20%20
          (bind _output_get (Variables|/Game/Sungsu/SS_Blueprints/BP_AssassinPlayer.BP_AssassinPlayer_C|SetplayerHP _player _result))
          (Development|PrintString (Utilities|String|ToString(Float) _output_get))
          (if (< _output_get 0.0)
            ;;[1 1 1] 사망
            (bind _output_get_2 (Variables|Default|SetrandAnimNum _returnvalue))
            (Class|IBPCombatSystem|IBPDie(Message) (Variables|Default|GettargetedEnemy) true _output_get_2)
            (Class|IBPCombatSystem|IBPDie(Message) _returnvalue_2 true _output_get_2)
            (else
              ;;[1 1 1] 일반 피격
              (bind _output_get_3 (Variables|Default|SetrandAnimNum _returnvalue))
              (Class|IBPCombatSystem|IBPHit(Message) _returnvalue_2 true _output_get_3))))))))

(event EventIBPHit
  (params (bIBPHit :type Boolean) (IBPHit :type Integer))
  (if (not bIBPHit)
    (Variables|Default|SetplayerCombatState "NewEnumerator1")))

(fn AttackRangeTracer
  (bind _desiredtargetdir (Variables|Default|GetdesiredTargetDir))
  (Variables|Default|SetnearestEnemyDistance 5e+04)
  (bind (_outactors _returnvalue) (Collision|SphereOverlapActors (Transformation|GetActorLocation (Variables|Default|Getplayer)) 4e+02 (Variables|Default|GetTargetTraceType) "/Game/Enemy/AIEnemy/AIEnemy.AIEnemy_C"))
  (if _returnvalue
    (for _array_element _outactors
      (bind _asaienemy (Utilities|Casting|CastToAIEnemy _array_element))
      (if (< (Math|Vector|VectorLength (- (Transformation|GetActorLocation _array_element) (Variables|Default|GetdesiredTargetDir))) (Variables|Default|GetnearestEnemyDistance))
        (Variables|Default|SetnearestEnemyDistance (Math|Vector|VectorLength (- (Transformation|GetActorLocation _array_element) (Variables|Default|GetdesiredTargetDir))))
        (Variables|Default|SettargetedEnemy _asaienemy)))
    (Class|KismetSystemLibrary|CapsuleTraceSingleforObjects _desiredtargetdir _desiredtargetdir 5e+01 4e+01 (Variables|Default|GetTargetTraceType) false 0 "ForOneFrame" true)
    (else
      (Variables|Default|SetnearestEnemyDistance 5e+04)
      (Variables|Default|SetplayerCombatState "NewEnumerator0")
      (Variables|Default|SetbInCombat false)
      (Variables|Default|SettargetedEnemy 0))))