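; Player stealth component that tracks whether enemies sense the player and whether assassination is allowed.
; Tick keeps CanAssassinate true in the stealth state; interface events play sounds for caution and detection, and detection clears that flag.
; The sensed event is built to record enemies and their offsets and enter Sensed, but MessageSendEnemy is set to None first, blocking that branch.
; Losing detection clears both lists and restores stealth.
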(event EventBeginPlay
  (Variables|Default|SetStealthstate "NewEnumerator5"))

(event EventTick
  (params (DeltaSeconds :type Float%20%28single-precision%29))
  (switch Utilities|FlowControl|Switch|SwitchonEBP_PalyerStealthState (Variables|Default|GetStealthstate)
    (:NewEnumerator5
      (Variables|Default|SetbCanAssassinate true))
    (:NewEnumerator0
      (if (Variables|Default|GetbIsSensed)
        _))))

(event EventIBPAISensedPlayer
  (params (bIBPIsSensed :type Boolean))
  (bind _sensedenemies (Variables|Default|GetsensedEnemies))
  ;[1 1 1] 감지 메세지 수신
  (bind _output_get (Variables|Default|SetbIsSensed bIBPIsSensed))
  (if _output_get
    (bind _output_get_2 (Variables|Default|SetmessageSendEnemy 0))
    (Utilities|IsValid _output_get_2
      (:Is%20Valid
        (Utilities|Array|Add _sensedenemies _output_get_2)
        (for _array_element _sensedenemies
          (Utilities|Array|Add (Variables|Default|GetenemyLoc) (- (Transformation|GetActorLocation _array_element) (Transformation|GetActorLocation (Components|GetOwner)))))
        (Variables|Default|SetStealthstate "NewEnumerator0")
        (Audio|PlaySound2D 0 1.0 1.0 0.0 0 0)))
    (else
      (Utilities|Array|Clear (Variables|Default|GetsensedEnemies))
      (Utilities|Array|Clear (Variables|Default|GetenemyLoc))
      (Variables|Default|SetStealthstate "NewEnumerator5"))))

(event EventIBPCaution
  (params (bIBPCautionState :type Boolean))
  (Audio|PlaySound2D 0 1.0 1.0 0.0 0 0))

(event EventIBPDetected
  (params (bIBPDetected :type Boolean))
  (Audio|PlaySound2D 0 1.0 1.0 0.0 0 0)
  (Variables|Default|SetbCanAssassinate false))