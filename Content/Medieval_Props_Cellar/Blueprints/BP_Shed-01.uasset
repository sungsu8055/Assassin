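; BP_Shed-01 is a modular shed prop from the cellar props set, with optional walls, roof and pillars.
; The Construction Script feeds five booleans (three walls, roof, pillars) into a shared EnabledDisabledMacro, one per static mesh component, to toggle visibility and collision.
; The event graph holds only disabled placeholder events, so it adds no runtime logic.
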(event EventBeginPlay)

(event EventActorBeginOverlap
  (params (OtherActor :type Actor%20Object%20Reference)))

(event EventTick
  (params (DeltaSeconds :type Float%20%28single-precision%29)))

(fn ConstructionScript
  (Utilities|FlowControl|Sequence
    (:then_0
      ;[1 1 1] Enable/disable. Macro (Visibility and Enable/Disable collision)
      (Utilities|Enabled/DisabledMacro (Variables|Modifiers|GetWall%201%20Enabled) (Variables|Default|GetStaticMeshComponent01)))
    (:then_1
      (Utilities|Enabled/DisabledMacro (Variables|Modifiers|GetWall%202%20Enabled) (Variables|Default|GetStaticMeshComponent03)))
    (:then_2
      (Utilities|Enabled/DisabledMacro (Variables|Modifiers|GetWall%203%20Enabled) (Variables|Default|GetStaticMeshComponent02)))
    (:then_3
      (Utilities|Enabled/DisabledMacro (Variables|Modifiers|GetRoof%20Enabled) (Variables|Default|GetStaticMeshComponent04)))
    (:then_4
      (Utilities|Enabled/DisabledMacro (Variables|Modifiers|GetPillars%20Enabled) (Variables|Default|GetStaticMeshComponent0)))))