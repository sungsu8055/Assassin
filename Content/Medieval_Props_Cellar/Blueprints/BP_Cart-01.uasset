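; Modular medieval cart prop whose parts can be toggled per instance.
; The Construction Script runs a sequence over nine static mesh components: base, upper part, shafts, front axle, four wheels and additional elements.
; Each part's boolean sets its visibility and switches its collision between QueryAndPhysics and NoCollision, so hidden parts do not block.
; It has no runtime logic, as the event graph holds only disabled placeholder events.
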(event EventBeginPlay)

(event EventActorBeginOverlap
  (params (OtherActor :type Actor%20Object%20Reference)))

(event EventTick
  (params (DeltaSeconds :type Float%20%28single-precision%29)))

(fn ConstructionScript
  (bind _staticmeshcomponent05 (Variables|Default|GetStaticMeshComponent05))
  (bind _cart_wheel_4_enabled (Variables|Modifiers|GetCart%20Wheel%204%20Enabled))
  (bind _staticmeshcomponent01 (Variables|Default|GetStaticMeshComponent01))
  (bind _cart_base_enabled (Variables|Modifiers|GetCart%20Base%20Enabled))
  (bind _staticmeshcomponent08 (Variables|Default|GetStaticMeshComponent08))
  (bind _cart_wheel_3_enabled (Variables|Modifiers|GetCart%20Wheel%203%20Enabled))
  (bind _staticmeshcomponent03 (Variables|Default|GetStaticMeshComponent03))
  (bind _cart_front_axle_enabled (Variables|Modifiers|GetCart%20Front%20axle%20Enabled))
  (bind _staticmeshcomponent02 (Variables|Default|GetStaticMeshComponent02))
  (bind _cart_up_enabled (Variables|Modifiers|GetCart%20Up%20Enabled))
  (bind _staticmeshcomponent04 (Variables|Default|GetStaticMeshComponent04))
  (bind _cart_shafts_enabled (Variables|Modifiers|GetCart%20Shafts%20Enabled))
  (bind _staticmeshcomponent07 (Variables|Default|GetStaticMeshComponent07))
  (bind _cart_wheel_1_enabled (Variables|Modifiers|GetCart%20Wheel%201%20Enabled))
  (bind _staticmeshcomponent06 (Variables|Default|GetStaticMeshComponent06))
  (bind _cart_wheel_2_enabled (Variables|Modifiers|GetCart%20Wheel%202%20Enabled))
  (bind _staticmeshcomponent0 (Variables|Default|GetStaticMeshComponent0))
  (bind _cart_additional_elements_enabled (Variables|Modifiers|GetCart%20Additional%20elements%20Enabled))
  (Utilities|FlowControl|Sequence
    (:then_0
      ;[1 1 1] Set Visibility objects
      (Rendering|SetVisibility _staticmeshcomponent02 _cart_up_enabled false)
      ;[1 1 1] Collision Enable/Disable
      (if _cart_up_enabled
        (Collision|SetCollisionEnabled _staticmeshcomponent02 "QueryAndPhysics")
        (else
          (Collision|SetCollisionEnabled _staticmeshcomponent02 "NoCollision"))))
    (:then_1
      (Rendering|SetVisibility _staticmeshcomponent04 _cart_shafts_enabled false)
      (if _cart_shafts_enabled
        (Collision|SetCollisionEnabled _staticmeshcomponent04 "QueryAndPhysics")
        (else
          (Collision|SetCollisionEnabled _staticmeshcomponent04 "NoCollision"))))
    (:then_2
      (Rendering|SetVisibility _staticmeshcomponent07 _cart_wheel_1_enabled false)
      (if _cart_wheel_1_enabled
        (Collision|SetCollisionEnabled _staticmeshcomponent07 "QueryAndPhysics")
        (else
          (Collision|SetCollisionEnabled _staticmeshcomponent07 "NoCollision"))))
    (:then_3
      (Rendering|SetVisibility _staticmeshcomponent06 _cart_wheel_2_enabled false)
      (if _cart_wheel_2_enabled
        (Collision|SetCollisionEnabled _staticmeshcomponent06 "QueryAndPhysics")
        (else
          (Collision|SetCollisionEnabled _staticmeshcomponent06 "NoCollision"))))
    (:then_4
      (Rendering|SetVisibility _staticmeshcomponent08 _cart_wheel_3_enabled false)
      (if _cart_wheel_3_enabled
        (Collision|SetCollisionEnabled _staticmeshcomponent08 "QueryAndPhysics")
        (else
          (Collision|SetCollisionEnabled _staticmeshcomponent08 "NoCollision"))))
    (:then_5
      (Rendering|SetVisibility _staticmeshcomponent05 _cart_wheel_4_enabled false)
      (if _cart_wheel_4_enabled
        (Collision|SetCollisionEnabled _staticmeshcomponent05 "QueryAndPhysics")
        (else
          (Collision|SetCollisionEnabled _staticmeshcomponent05 "NoCollision"))))
    (:then_6
      (Rendering|SetVisibility _staticmeshcomponent03 _cart_front_axle_enabled false)
      (if _cart_front_axle_enabled
        (Collision|SetCollisionEnabled _staticmeshcomponent03 "QueryAndPhysics")
        (else
          (Collision|SetCollisionEnabled _staticmeshcomponent03 "NoCollision"))))
    (:then_7
      (Rendering|SetVisibility _staticmeshcomponent0 _cart_additional_elements_enabled false)
      (if _cart_additional_elements_enabled
        (Collision|SetCollisionEnabled _staticmeshcomponent0 "QueryAndPhysics")
        (else
          (Collision|SetCollisionEnabled _staticmeshcomponent0 "NoCollision"))))
    (:then_8
      (Rendering|SetVisibility _staticmeshcomponent01 _cart_base_enabled false)
      (if _cart_base_enabled
        (Collision|SetCollisionEnabled _staticmeshcomponent01 "QueryAndPhysics")
        (else
          (Collision|SetCollisionEnabled _staticmeshcomponent01 "NoCollision"))))))